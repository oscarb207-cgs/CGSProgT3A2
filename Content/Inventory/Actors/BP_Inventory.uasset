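; BP_Inventory is an actor that displays the player's inventory grid through a widget component.
; After a short delay on BeginPlay it caches the WBP_InventoryGrid and draws a long-lived debug point, converting randomly picked slot geometry into world space.
; ShowInventory resets all slot states, then uses the player's AC_Inventory to compute each item's rotated shape coordinates and changes the state of the slots they cover.
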(event Custom|ShowInventory
  (bind _returnvalue (Game|GetPlayerCharacter 0))
  (bind _inventorygridwidget (Variables|Default|GetInventoryGridWidget))
  (bind _returnvalue_2 (Actor|GetComponentbyClass _returnvalue "/Game/Inventory/Components/AC_Inventory.AC_Inventory_C"))
  (Default|SetAllSlotStates _inventorygridwidget "NewEnumerator0")
  (for _array_element (Variables|/Game/Inventory/Components/AC_Inventory.AC_Inventory_C|GetInventoryArray _returnvalue_2)
    (bind _rotatedcoords (Default|GetRotatedShapeCoordinates _returnvalue_2 (.Coordinates (Utilities|Struct|BreakST_InventoryItem _array_element)) (.Rotation (Utilities|Struct|BreakST_InventoryItem _array_element)) (.Shape (Utilities|Struct|BreakST_InventoryItem _array_element))))
    (for _array_element_2 _rotatedcoords
      (Default|ChangeSlotState (.Value (Utilities|Map|Find (Variables|/Game/Inventory/Widgets/WBP_InventoryGrid.WBP_InventoryGrid_C|GetSlotsMap _inventorygridwidget) _array_element_2)) "NewEnumerator5"))))

(event EventBeginPlay
  (bind _widget (Variables|Default|GetWidget))
  (Utilities|FlowControl|Delay 0.2)
  (bind _aswbp_inventory_grid (Utilities|Casting|CastToWBP_InventoryGrid (UserInterface|GetUserWidgetObject _widget)))
  (Variables|Default|SetInventoryGridWidget _aswbp_inventory_grid)
  (bind _values (Utilities|Map|Values (Variables|/Game/Inventory/Widgets/WBP_InventoryGrid.WBP_InventoryGrid_C|GetSlotsMap _aswbp_inventory_grid)))
  (Rendering|Debug|DrawDebugPoint (Math|Transform|TransformLocation (Transformation|GetWorldTransform _widget) (Math|Vector|MakeVector 0.0 (.X (Math|Vector2D|BreakVector2D (Class|KismetMathLibrary|Negated2D (Class|SlateBlueprintLibrary|VectorLocaltoAbsolute (Class|Widget|GetCachedGeometry (.OutItem (Utilities|Array|Random _values))) (+ (/ (Class|SlateBlueprintLibrary|GetLocalSize (Class|Widget|GetCachedGeometry (.OutItem (Utilities|Array|Random _values)))) 2.0) (Class|SlateBlueprintLibrary|GetLocalTopLeft (Class|Widget|GetCachedGeometry (.OutItem (Utilities|Array|Random _values))))))))) (.Y (Math|Vector2D|BreakVector2D (Class|KismetMathLibrary|Negated2D (Class|SlateBlueprintLibrary|VectorLocaltoAbsolute (Class|Widget|GetCachedGeometry (.OutItem (Utilities|Array|Random _values))) (+ (/ (Class|SlateBlueprintLibrary|GetLocalSize (Class|Widget|GetCachedGeometry (.OutItem (Utilities|Array|Random _values)))) 2.0) (Class|SlateBlueprintLibrary|GetLocalTopLeft (Class|Widget|GetCachedGeometry (.OutItem (Utilities|Array|Random _values))))))))))) 4.0 "(R=1.000000,G=0.000000,B=0.014216,A=1.000000)" 1e+09))

(fn ConstructionScript)
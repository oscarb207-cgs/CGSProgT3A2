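; BP_PickupItem is a world pickup that transfers its ItemData into the inventory of an actor that overlaps it.
; On BeginPlay it sets its static mesh from the item's data asset.
; When its sphere is overlapped, it looks for AC_Inventory on the other actor and calls TryAddToInventory.
; The returned value becomes the remaining quantity, and the pickup destroys itself once none is left.
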(event OnComponentBeginOverlap(Sphere)
  (params (OverlappedComponent :type Primitive%20Component%20Object%20Reference) (OtherActor :type Actor%20Object%20Reference) (OtherComp :type Primitive%20Component%20Object%20Reference) (OtherBodyIndex :type Integer) (bFromSweep :type Boolean) (SweepResult :type Hit%20Result%20Structure%20%28by%20ref%29))
  (bind _returnvalue (Actor|GetComponentbyClass OtherActor "/Game/Inventory/Components/AC_Inventory.AC_Inventory_C"))
  (bind _itemdata (Variables|Default|GetItemData))
  (Utilities|IsValid _returnvalue
    (:Is%20Valid
      (bind _remainingquantity (Class|BPIInventory|TryAddtoInventory(Message) _returnvalue _itemdata))
      (bind _structout (Utilities|Struct|SetmembersinST_PreInventoryData _itemdata _remainingquantity))
      (if (<= (.quantity _structout) 0)
        (Actor|DestroyActor)))))

(event EventBeginPlay
  (Components|StaticMesh|SetStaticMesh (Variables|Default|GetStaticMesh) (Variables|/Game/Inventory/DataAssets/DA_InventoryItem.DA_InventoryItem_C|GetItemMesh (.dataasset (Variables|Default|GetItemData)))))

(fn ConstructionScript)
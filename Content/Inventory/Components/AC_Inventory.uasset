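; Grid inventory component that stores multi-cell shaped items, with stacking and removal by GUID.
; BeginPlay fills a coordinate-to-occupied map, which placement checks use to reject taken or out-of-grid cells.
; Adding expands data-asset info into a full item, tops up matching stacks, then puts any remainder in the first slot that fits, trying four rotations.
; It returns the quantity left over; removal frees the item's rotated footprint.
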(event EventBeginPlay
  (CallFunction|InventoryInitialisation))

(fn InventoryInitialisation
  (bind _slot (Utilities|ForEachSlot (Variables|Init|GetTotalSlots) (Variables|Init|GetRowLength))
    (:Loop%20Body
      (Utilities|Map|Add (Variables|Default|GetCoordinateAvailabilityMap) _slot false))))

(fn TryAddItem
  (params (ItemData :type ST%20Pre%20Inventory%20Data%20Structure))
  (bind _fulldata (CallFunction|ConvertItemDatatoFull ItemData))
  (bind _output_get (LocalVariables|SetLocalItemData _fulldata))
  (Utilities|FlowControl|Sequence
    (:then_0
      (bind _returnitemdata (CallFunction|TryMergeItem _output_get))
      (LocalVariables|SetLocalItemData _returnitemdata))
    (:then_1
      (if (> (Utilities|Struct|BreakST_InventoryItem (LocalVariables|GetLocalItemData)) 0)
        (bind _slot (Utilities|ForEachSlot (Variables|Init|GetTotalSlots) (Variables|Init|GetRowLength))
          (:Loop%20Body
            (bind (_canadd _rotationused) (CallFunction|CanAddtoSlot _slot (.shape (LocalVariables|GetLocalItemData))))
            (if _canadd
              (CallFunction|AddItemtoInventory (Utilities|Struct|MakeST_InventoryItem (.shape (LocalVariables|GetLocalItemData)) _slot _rotationused (.name (LocalVariables|GetLocalItemData)) (.mesh (LocalVariables|GetLocalItemData)) (.currentquantity (LocalVariables|GetLocalItemData)) (.maxquantity (LocalVariables|GetLocalItemData)) (.dataasset (LocalVariables|GetLocalItemData)) (.itemguid (LocalVariables|GetLocalItemData))))
              (return 0)))
          (:Completed
            (return (Utilities|Struct|BreakST_InventoryItem (LocalVariables|GetLocalItemData)))))
        (else
          (return (Utilities|Struct|BreakST_InventoryItem (LocalVariables|GetLocalItemData))))))))

(fn ConvertItemDatatoFull
  (params (PreData :type ST%20Pre%20Inventory%20Data%20Structure))
  (bind (_dataasset _quantity) (Utilities|Struct|BreakST_PreInventoryData PreData))
  (return (Utilities|Struct|MakeST_InventoryItem (Variables|/Game/Inventory/DataAssets/DA_InventoryItem.DA_InventoryItem_C|GetShape _dataasset) "(X=-1.000000,Y=-1.000000)" 0.0 (Variables|/Game/Inventory/DataAssets/DA_InventoryItem.DA_InventoryItem_C|GetName _dataasset) (Variables|/Game/Inventory/DataAssets/DA_InventoryItem.DA_InventoryItem_C|GetItemMesh _dataasset) _quantity (Variables|/Game/Inventory/DataAssets/DA_InventoryItem.DA_InventoryItem_C|GetMaxQuantity _dataasset) _dataasset (Guid|NewGuid))))

(fn GetRotatedShapeCoordinates
  (params (Coordinates :type Vector%202D%20Structure) (Rotation :type Float%20%28double-precision%29) (Shape :type Array%20of%20Vector%202D%20Structures))
  (bind _rotatedshape (Utilities|Rotate2DArray Shape Rotation))
  (bind _output_get (LocalVariables|SetShapeInUse _rotatedshape))
  (for (_array_element _array_index) _output_get
    (Utilities|Array|SetArrayElem _output_get _array_index (+ _array_element Coordinates)))
  (return (LocalVariables|GetShapeInUse)))

(fn AddItemtoInventory
  (params (ItemData :type ST%20Inventory%20Item%20Structure))
  (bind (_shape _coordinates _rotation) (Utilities|Struct|BreakST_InventoryItem ItemData))
  (bind _rotatedcoords (CallFunction|GetRotatedShapeCoordinates _coordinates _rotation _shape))
  (for _array_element _rotatedcoords
    (Utilities|Map|Add (Variables|Default|GetCoordinateAvailabilityMap) _array_element true))
  (Utilities|Array|Add (Variables|Default|GetInventoryArray) ItemData))

(fn CanAddtoSlot
  (params (Coordinates :type Vector%202D%20Structure) (Shape :type Array%20of%20Vector%202D%20Structures))
  (for _array_element (Utilities|Array|MakeArray 0.0 9e+01 1.8e+02 -9e+01)
    (bind _rotatedcoords (CallFunction|GetRotatedShapeCoordinates Coordinates _array_element Shape))
    (if (CallFunction|AreSlotsAvailable _rotatedcoords)
      (return true _array_element)))
  (return false 0.0))

(fn AreSlotsAvailable
  (params (Slots :type Array%20of%20Vector%202D%20Structures))
  (for _array_element Slots
    (if (.ReturnValue (Utilities|Map|Find (Variables|Default|GetCoordinateAvailabilityMap) _array_element))
      (if (.Value (Utilities|Map|Find (Variables|Default|GetCoordinateAvailabilityMap) _array_element))
        (return false))
      (else
        (return false))))
  (return true))

(fn RemoveItemfromInventory
  (params (ItemData :type ST%20Inventory%20Item%20Structure))
  (bind _itemindex (CallFunction|FindItembyGUID (.ItemGUID (Utilities|Struct|BreakST_InventoryItem ItemData))))
  (if (== _itemindex -1)
    (return false)
    (else
      (bind _rotatedcoords (CallFunction|GetRotatedShapeCoordinates (.Coordinates (Utilities|Struct|BreakST_InventoryItem (Utilities|Array|Get(acopy) (Variables|Default|GetInventoryArray) _itemindex))) (.Rotation (Utilities|Struct|BreakST_InventoryItem (Utilities|Array|Get(acopy) (Variables|Default|GetInventoryArray) _itemindex))) (.Shape (Utilities|Struct|BreakST_InventoryItem (Utilities|Array|Get(acopy) (Variables|Default|GetInventoryArray) _itemindex)))))
      (for _array_element _rotatedcoords
        (Utilities|Map|Add (Variables|Default|GetCoordinateAvailabilityMap) _array_element false))
      (Guid|InvalidateGuid (.ItemGUID (Utilities|Struct|BreakST_InventoryItem (Utilities|Array|Get(acopy) (Variables|Default|GetInventoryArray) _itemindex))))
      (Utilities|Array|RemoveIndex (Variables|Default|GetInventoryArray) _itemindex)
      (return true))))

(fn FindItembyGUID
  (params (GUID :type Guid%20Structure))
  (for (_array_element _array_index) (Variables|Default|GetInventoryArray)
    (if (== (.ItemGUID (Utilities|Struct|BreakST_InventoryItem _array_element)) GUID)
      (return _array_index)))
  (return -1))

(fn TryMergeItem
  (params (ItemData :type ST%20Inventory%20Item%20Structure))
  (LocalVariables|SetLocalItemData ItemData)
  (bind (_array_element _array_index) (Utilities|Array|ForEachLoopwithBreak (Variables|Default|GetInventoryArray) :!label _label)
    (:LoopBody
      (if (and (< (.CurrentQuantity (Utilities|Struct|BreakST_InventoryItem _array_element)) (.MaxQuantity (Utilities|Struct|BreakST_InventoryItem _array_element))) (== (.DataAsset (Utilities|Struct|BreakST_InventoryItem _array_element)) (.DataAsset (Utilities|Struct|BreakST_InventoryItem (LocalVariables|GetLocalItemData)))))
        (bind _output_get (LocalVariables|SetPreCurrentQuant (.CurrentQuantity (Utilities|Struct|BreakST_InventoryItem _array_element))))
        (bind _structout (Utilities|Struct|SetmembersinST_InventoryItem _array_element (Math|Integer|Clamp(Integer) (+ _output_get (.CurrentQuantity (Utilities|Struct|BreakST_InventoryItem (LocalVariables|GetLocalItemData)))) 0 (.MaxQuantity (Utilities|Struct|BreakST_InventoryItem _array_element)))))
        (Utilities|Array|SetArrayElem (Variables|Default|GetInventoryArray) _array_index _structout)
        (bind _structout_2 (Utilities|Struct|SetmembersinST_InventoryItem (LocalVariables|GetLocalItemData) (- (Utilities|Struct|BreakST_InventoryItem (LocalVariables|GetLocalItemData)) (- (Utilities|Struct|BreakST_InventoryItem _structout) _output_get))))
        (bind _output_get_2 (LocalVariables|SetLocalItemData _structout_2))
        (if (<= (Utilities|Struct|BreakST_InventoryItem _output_get_2) 0)
          (goto _label Break))))
    (:Completed
      (return (LocalVariables|GetLocalItemData)))))

(fn TryAddtoInventory
  (params (ItemData :type ST%20Pre%20Inventory%20Data%20Structure))
  (bind _quantityremaining (CallFunction|TryAddItem ItemData))
  (return _quantityremaining))